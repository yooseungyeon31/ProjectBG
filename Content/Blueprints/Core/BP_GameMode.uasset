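; Game mode that populates the level with randomized loot at BeginPlay.
; For each DT_ItemGroupLocations row, it spawns a BP_ItemGroup, rolls an item count and gets that many random transforms from the group.
; It re-rolls item types until unique within the group, then picks an ID per type and spawns BP_TestItem actors.
; Count, type and ID rolls are weighted by repeating DataTable entries by Percent before random picks.
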(event `self.ReceiveBeginPlay`
  (`self.GenerateItems`))

(fn `GenerateItems`
  (locals (ItemTypeArr :type "Array of /Game/Blueprints/Datas/Enum/Item/E_ItemType Enum") (SpawnItemArr :type "Array of /Game/Blueprints/Datas/Struct/ItemGeneration/ST_SpawnItem Structure") (SpawnTransforms :type "Array of Transform Structure") (ItemGroupRef :type "/Game/Blueprints/Items/BP_ItemGroup Object Reference") (ItemType :type "/Game/Blueprints/Datas/Enum/Item/E_ItemType Enum") (SpawnID :type Name))
  ; datatable의 전체 로우네임 가져오기
  (bind _outrownames (`DataTableFunctionLibrary.GetDataTableRowNames` "/Game/Blueprints/Datas/DataTable/ItemGeneration/DT_ItemGroupLocations.DT_ItemGroupLocations"))
  (for _array_element _outrownames
    (bind _returnvalue (`|GetDataTableRow` "/Game/Blueprints/Datas/DataTable/ItemGeneration/DT_ItemGroupLocations.DT_ItemGroupLocations" _array_element)
      (:`then`
        (bind _returnvalue_2 (`|SpawnActorFromClass` "/Game/Blueprints/Items/BP_ItemGroup.BP_ItemGroup_C" (`KismetMathLibrary.MakeTransform` (break `/Game/Blueprints/Datas/Struct/ItemGeneration/ST_ItemGroupLocation` _returnvalue)) "Undefined" "MultiplyWithRoot" null null))
        (set `local.ItemGroupRef` _returnvalue_2)
        (`KismetArrayLibrary.Array_Clear` (`local.ItemTypeArr`))
        ; 아이템 그룹에 생성될 랜덤 아이템 개수 정하기
        (bind _number (`self.RandomItemNumber`))
        (set `local.SpawnTransforms` (`/Game/Blueprints/Items/BP_ItemGroup.GetRandomTransforms` (`local.ItemGroupRef`) _number))
        (for _ (range 1 (+ _number 1))
          ; 랜덤한 아이템 타입 정하기
          (bind _itemtype (`self.RandomItemType` :!label _label))
          ; 아이템 중복 방지
          (if (== (`KismetArrayLibrary.Array_Find` (`local.ItemTypeArr`) _itemtype) -1)
            (`KismetArrayLibrary.Array_Add` (`local.ItemTypeArr`) _itemtype)
            (else
              (goto _label))))
        (for _array_element_2 (`local.ItemTypeArr`)
          (bind _spawnitem (`self.RandomItemID` _array_element_2))
          (`KismetArrayLibrary.Array_Add` (`local.SpawnItemArr`) _spawnitem))
        (for (_array_element_3 _array_index) (`local.SpawnItemArr`)
          (set `local.ItemType` (break `/Game/Blueprints/Datas/Struct/ItemGeneration/ST_SpawnItem` _array_element_3))
          (set `local.SpawnID` (`.ID_5_48815FF64509AD45D0CDF486753D02B1` (break `/Game/Blueprints/Datas/Struct/ItemGeneration/ST_SpawnItem` _array_element_3)))
          (`|SpawnActorFromClass` "/Game/Blueprints/BP_TestItem.BP_TestItem_C" (`|GetArrayItem` (`local.SpawnTransforms`) _array_index) "Undefined" "MultiplyWithRoot" null null))
        (`KismetArrayLibrary.Array_Clear` (`local.SpawnItemArr`))))))

(fn `RandomItemID`
  (params (ItemType :type "/Game/Blueprints/Datas/Enum/Item/E_ItemType Enum" :default "NewEnumerator0"))
  (returns (SpawnItem :type "/Game/Blueprints/Datas/Struct/ItemGeneration/ST_SpawnItem Structure"))
  (locals (ItemArr :type "Array of /Game/Blueprints/Datas/Struct/ItemGeneration/ST_SpawnItem Structure"))
  (bind _returnvalue (select `/Game/Blueprints/Datas/Enum/Item/E_ItemType` (`local.ItemType`) :`NewEnumerator0` "/Game/Blueprints/Datas/DataTable/ItemGeneration/DT_WeaponProbability.DT_WeaponProbability" :`NewEnumerator1` "/Game/Blueprints/Datas/DataTable/ItemGeneration/DT_WeaponAccProbability.DT_WeaponAccProbability" :`NewEnumerator2` "/Game/Blueprints/Datas/DataTable/ItemGeneration/DT_AmmoProbability.DT_AmmoProbability" :`NewEnumerator3` "/Game/Blueprints/Datas/DataTable/ItemGeneration/DT_HealthProbability.DT_HealthProbability" :`NewEnumerator4` "/Game/Blueprints/Datas/DataTable/ItemGeneration/DT_BoostProbability.DT_BoostProbability" :`NewEnumerator5` "/Game/Blueprints/Datas/DataTable/ItemGeneration/DT_HelmetProbability.DT_HelmetProbability" :`NewEnumerator6` "/Game/Blueprints/Datas/DataTable/ItemGeneration/DT_VestProbability.DT_VestProbability" :`NewEnumerator7` "/Game/Blueprints/Datas/DataTable/ItemGeneration/DT_BackpackProbability.DT_BackpackProbability" :!type "DataTable Object Reference"))
  (`|ExecutionSequence`
    (:`then_0`
      (bind _outrownames (`DataTableFunctionLibrary.GetDataTableRowNames` _returnvalue))
      (for _array_element _outrownames
        (bind _returnvalue_2 (`|GetDataTableRow` _returnvalue _array_element)
          (:`then`
            (for _ (range 1 (+ (`.Percent_2_A6D6D3594B08A77510660AAE1B166266` (break `/Game/Blueprints/Datas/Struct/ItemGeneration/ST_ItemProbability` _returnvalue_2)) 1))
              (`KismetArrayLibrary.Array_Add` (`local.ItemArr`) (make `/Game/Blueprints/Datas/Struct/ItemGeneration/ST_SpawnItem` (`local.ItemType`) _array_element)))))))
    (:`then_1`
      (return (`KismetArrayLibrary.Array_Random` (`local.ItemArr`))))))

(fn `RandomItemNumber`
  (returns (Number :type Integer))
  (locals (NumberArr :type "Array of Integer"))
  ; 데이터 테이블에서 각 숫자가 나올 확률 가져오기
  (bind _outrownames (`DataTableFunctionLibrary.GetDataTableRowNames` "/Game/Blueprints/Datas/DataTable/ItemGeneration/DT_NumberProbabilitys.DT_NumberProbabilitys"))
  (for _array_element _outrownames
    (bind _returnvalue (`|GetDataTableRow` "/Game/Blueprints/Datas/DataTable/ItemGeneration/DT_NumberProbabilitys.DT_NumberProbabilitys" _array_element)
      (:`then`
        ; 각 숫자를 퍼센트 만큼 배열에 채워주기
        (for _ (range 1 (+ (break `/Game/Blueprints/Datas/Struct/ItemGeneration/ST_NumberProbablity` _returnvalue) 1))
          (`KismetArrayLibrary.Array_Add` (`local.NumberArr`) (`.Number_4_22142A8B4DC7598D010353B90DC0AE45` (break `/Game/Blueprints/Datas/Struct/ItemGeneration/ST_NumberProbablity` _returnvalue)))))))
  (return (`KismetArrayLibrary.Array_Random` (`local.NumberArr`))))

(fn `RandomItemType`
  (returns (ItemType :type "/Game/Blueprints/Datas/Enum/Item/E_ItemType Enum"))
  (locals (ItemTypeArr :type "Array of /Game/Blueprints/Datas/Enum/Item/E_ItemType Enum"))
  (bind _outrownames (`DataTableFunctionLibrary.GetDataTableRowNames` "/Game/Blueprints/Datas/DataTable/ItemGeneration/DT_ItemTypeProbability.DT_ItemTypeProbability"))
  (for _array_element _outrownames
    (bind _returnvalue (`|GetDataTableRow` "/Game/Blueprints/Datas/DataTable/ItemGeneration/DT_ItemTypeProbability.DT_ItemTypeProbability" _array_element)
      (:`then`
        (for _ (range 1 (+ (break `/Game/Blueprints/Datas/Struct/ItemGeneration/ST_ItemTypeProbability` _returnvalue) 1))
          (`KismetArrayLibrary.Array_Add` (`local.ItemTypeArr`) (`.ItemType_5_52F7E2CB446372736F064AA895F31D1A` (break `/Game/Blueprints/Datas/Struct/ItemGeneration/ST_ItemTypeProbability` _returnvalue)))))))
  (return (`KismetArrayLibrary.Array_Random` (`local.ItemTypeArr`))))

(fn `UserConstructionScript`)